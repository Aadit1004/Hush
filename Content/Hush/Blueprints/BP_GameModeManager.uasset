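; Manager for Hush's game state that handles starting the level and resetting the flashlight.
; On BeginPlay it stores the first BP_Flashlight's transform, sets an initial game state and caches the player character.
; Resetting destroys the flashlight, respawns it at the saved transform and clears the player's flashlight flags.
; StartGame opens BackroomsLevel, while ResetGame and GameOver are empty stubs.
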(event Custom|SaveFlashlightReference
  (bind _outactors (Actor|GetAllActorsOfClass "/Game/Hush/Blueprints/BP_Flashlight.BP_Flashlight_C"))
  (bind _output_get (Variables|Default|SetFlashlightRef (Utilities|Array|Get(acopy) _outactors)))
  (Variables|Default|SetFlashlightProperties (Math|Transform|MakeTransform (.location (Transformation|GetActorTransform _output_get)) (.rotation (Transformation|GetActorTransform _output_get)) (.scale (Transformation|GetActorTransform _output_get)))))

(event EventBeginPlay
  (CallFunction|SaveFlashlightReference)
  (Variables|Default|SetEGameState "NewEnumerator0")
  (bind _asbp_third_person_character (Utilities|Casting|CastToBP_ThirdPersonCharacter (Game|GetPlayerCharacter 0)))
  (Variables|Default|SetPlayerCharacterRef _asbp_third_person_character))

(event EventTick
  (params (DeltaSeconds :type Float%20%28single-precision%29)))

(fn ConstructionScript)

(fn ResetFlashlight
  (Actor|DestroyActor (Variables|Default|GetFlashlightRef))
  (bind _returnvalue (Game|SpawnActorfromClass "/Game/Hush/Blueprints/BP_Flashlight.BP_Flashlight_C" (Variables|Default|GetFlashlightProperties) "Undefined" "MultiplyWithRoot" 0 0))
  (Variables|Default|SetFlashlightRef _returnvalue)
  (bind _asbp_third_person_character (Utilities|Casting|CastToBP_ThirdPersonCharacter (Game|GetPlayerCharacter 0)))
  (Variables|/Game/ThirdPerson/Blueprints/BP_ThirdPersonCharacter.BP_ThirdPersonCharacter_C|SetbHasFlashlight _asbp_third_person_character false)
  (Variables|/Game/ThirdPerson/Blueprints/BP_ThirdPersonCharacter.BP_ThirdPersonCharacter_C|SetbIsFlashlightOn _asbp_third_person_character false))

(fn ResetGame)

(fn ResetActorsandLocation
  (CallFunction|ResetFlashlight))

(fn StartGame
  (Game|OpenLevel(byName) "BackroomsLevel"))

(fn GameOver)
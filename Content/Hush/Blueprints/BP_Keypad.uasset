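; BP_Keypad is an interactable keypad that lets the player unlock a door exit by entering a code, available only after the lights are repaired.
; Interacting opens a WB_Keypad widget, disables movement and switches to UI-only input until HideKeypadUI restores gameplay control.
; A box overlap toggles a billboard and player prompt.
; CorrectCode sets the player's CanLeaveDoor flag, after which the keypad no longer opens.
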(event OnComponentBeginOverlap(Box)
  (params (OverlappedComponent :type Primitive%20Component%20Object%20Reference) (OtherActor :type Actor%20Object%20Reference) (OtherComp :type Primitive%20Component%20Object%20Reference) (OtherBodyIndex :type Integer) (bFromSweep :type Boolean) (SweepResult :type Hit%20Result%20Structure%20%28by%20ref%29))
  (if (== OtherActor (Variables|Default|GetPlayerRef))
    (CallFunction|ShowUI)))

(event OnComponentEndOverlap(Box)
  (params (OverlappedComponent :type Primitive%20Component%20Object%20Reference) (OtherActor :type Actor%20Object%20Reference) (OtherComp :type Primitive%20Component%20Object%20Reference) (OtherBodyIndex :type Integer))
  (if (== (Variables|Default|GetPlayerRef) OtherActor)
    (CallFunction|HideUI)))

(event Custom|ShowUI
  (bind _playerref (Variables|Default|GetPlayerRef))
  (Rendering|SetVisibility (Variables|Default|GetBillboard) true false)
  (if (Variables|/Game/ThirdPerson/Blueprints/BP_ThirdPersonCharacter.BP_ThirdPersonCharacter_C|GetbHasRepaired _playerref)
    (Default|DisplayPrompt _playerref "NewEnumerator0")))

(event Custom|HideUI
  (bind _playerref (Variables|Default|GetPlayerRef))
  (Rendering|SetVisibility (Variables|Default|GetBillboard) false false)
  (if (Variables|/Game/ThirdPerson/Blueprints/BP_ThirdPersonCharacter.BP_ThirdPersonCharacter_C|GetbHasRepaired _playerref)
    (Default|HidePrompt _playerref "NewEnumerator0")))

(event Custom|HideKeypadUI
  (bind _returnvalue (Game|GetPlayerController 0))
  (Widget|RemovefromParent (Variables|Default|GetWB_Keypad))
  (Default|EnableMovement (Variables|Default|GetPlayerRef))
  (Input|SetInputModeGameOnly _returnvalue false)
  (Variables|/Script/Engine.PlayerController|SetbShowMouseCursor _returnvalue false)
  (CallFunction|ShowUI))

(event Custom|CorrectCode
  (Variables|/Game/ThirdPerson/Blueprints/BP_ThirdPersonCharacter.BP_ThirdPersonCharacter_C|SetbCanLeaveDoor (Variables|Default|GetPlayerRef) true))

(event EventBeginPlay
  (bind _asbp_third_person_character (Utilities|Casting|CastToBP_ThirdPersonCharacter (Game|GetPlayerCharacter 0)))
  (Variables|Default|SetPlayerRef _asbp_third_person_character)
  (bind _returnvalue (UserInterface|CreateWidget "/Game/Hush/UI/WB_Keypad.WB_Keypad_C"))
  (Variables|Default|SetWB_Keypad _returnvalue))

(event EventInteract
  (bind _returnvalue (Game|GetPlayerController 0))
  (if (Variables|/Game/ThirdPerson/Blueprints/BP_ThirdPersonCharacter.BP_ThirdPersonCharacter_C|GetbHasRepaired (Variables|Default|GetPlayerRef))
    (if (not (Variables|/Game/ThirdPerson/Blueprints/BP_ThirdPersonCharacter.BP_ThirdPersonCharacter_C|GetbCanLeaveDoor (Variables|Default|GetPlayerRef)))
      (UserInterface|Viewport|AddtoViewport (Variables|Default|GetWB_Keypad) 0)
      (Default|DisableMovement (Variables|Default|GetPlayerRef))
      (Input|SetInputModeUIOnly _returnvalue 0 "DoNotLock" false)
      (Variables|/Script/Engine.PlayerController|SetbShowMouseCursor _returnvalue true)
      (CallFunction|HideUI))
    (else
      (Development|PrintString "repair lights"))))

(fn ConstructionScript)
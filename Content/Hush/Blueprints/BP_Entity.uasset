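; BP_Entity is an AI pursuer that roams, chases the player and triggers the end-game screen when it catches them.
; Tick dispatches on a state enum to looping AIMoveTo calls, toward random reachable points or the player's updated location.
; Three collision volumes drive transitions: detection starts a chase, inner overlap means caught, and leaving the outer one resumes roaming.
; Caught repeatedly calls TriggerLoseScreen from Tick, which stops movement and shows WB_WinEndGame after a delay.
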(event OnComponentBeginOverlap(DetectionCollision)
  (params (OverlappedComponent :type Primitive%20Component%20Object%20Reference) (OtherActor :type Actor%20Object%20Reference) (OtherComp :type Primitive%20Component%20Object%20Reference) (OtherBodyIndex :type Integer) (bFromSweep :type Boolean) (SweepResult :type Hit%20Result%20Structure%20%28by%20ref%29))
  (if (Math|Boolean|ANDBoolean (== OtherActor (Variables|Default|GetPlayerRef)) (Variables|Default|GetisActive) (Variables|Default|GetisRoaming))
    (Variables|Default|SetisRoaming false)
    (Variables|Default|SetCurrentState "NewEnumerator1")
    (Development|PrintString "start chasing")))

(event OnComponentBeginOverlap(InnerDetectionCollision)
  (params (OverlappedComponent :type Primitive%20Component%20Object%20Reference) (OtherActor :type Actor%20Object%20Reference) (OtherComp :type Primitive%20Component%20Object%20Reference) (OtherBodyIndex :type Integer) (bFromSweep :type Boolean) (SweepResult :type Hit%20Result%20Structure%20%28by%20ref%29))
  (if (Math|Boolean|ANDBoolean (== OtherActor (Variables|Default|GetPlayerRef)) (Variables|Default|GetisActive) (Utilities|Enum|Equal(Enum) (Variables|Default|GetCurrentState) "NewEnumerator1"))
    (Variables|Default|SetCurrentState "NewEnumerator3")))

(event OnComponentEndOverlap(OuterDetectionCollision)
  (params (OverlappedComponent :type Primitive%20Component%20Object%20Reference) (OtherActor :type Actor%20Object%20Reference) (OtherComp :type Primitive%20Component%20Object%20Reference) (OtherBodyIndex :type Integer))
  (if (Math|Boolean|ANDBoolean (== OtherActor (Variables|Default|GetPlayerRef)) (Variables|Default|GetisActive) (Utilities|Enum|Equal(Enum) (Variables|Default|GetCurrentState) "NewEnumerator1"))
    (Variables|Default|SetCurrentState "NewEnumerator0")
    (Variables|Default|SetisChasing false)
    (Development|PrintString "Escaped Chasing")))

(event Custom|StartRoaming
  (Variables|Default|SetisRoaming true)
  (Variables|Default|SetCurrentState "NewEnumerator0")
  (AI|AIMoveTo self (.RandomLocation (AI|Navigation|GetRandomReachablePointinRadius (Transformation|GetActorLocation) 1.5e+03 0 0)) 0 5.0 false :!label _label
    (:OnSuccess
      (Utilities|FlowControl|Delay 0.2)
      (goto _label))))

(event Custom|TriggerLoseScreen
  (bind _returnvalue (Game|GetPlayerController 0))
  (Development|PrintString "Play Caught Cutsccene / STOP SOUNDS -> End Game")
  (CallFunction|StopMovement)
  (Utilities|FlowControl|Delay 2.0)
  (bind _returnvalue_2 (UserInterface|CreateWidget "/Game/Hush/UI/Menus/WB_WinEndGame.WB_WinEndGame_C"))
  (UserInterface|Viewport|AddtoViewport _returnvalue_2 0)
  (Variables|/Script/Engine.PlayerController|SetbShowMouseCursor _returnvalue true)
  (Input|SetInputModeUIOnly _returnvalue 0 "DoNotLock" false))

(event Custom|StopMovement
  (bind _self self)
  (AI|AIMoveTo _self (Transformation|GetActorLocation _self) 0 5.0 false
    (:OnSuccess
      (Variables|Default|SetisActive false))))

(event Custom|StartChasing
  (Variables|Default|SetisChasing true)
  (AI|AIMoveTo self (Variables|Default|GetplayerLoc) 0 5.0 false :!label _label
    (:OnSuccess
      (goto _label))))

(event EventBeginPlay
  (bind _asbp_third_person_character (Utilities|Casting|CastToBP_ThirdPersonCharacter (Game|GetPlayerCharacter 0)))
  (Variables|Default|SetPlayerRef _asbp_third_person_character))

(event EventTick
  (params (DeltaSeconds :type Float%20%28single-precision%29))
  (bind _playerref (Variables|Default|GetPlayerRef))
  (bind _returnvalue (Transformation|GetActorLocation _playerref))
  (switch Utilities|FlowControl|Switch|SwitchonEEntityState (Variables|Default|GetCurrentState)
    (:NewEnumerator0
      (if (not (Variables|Default|GetisRoaming))
        (CallFunction|StartRoaming)))
    (:NewEnumerator1
      (if (Variables|Default|GetisChasing)
        (Variables|Default|SetplayerLoc _returnvalue)
        (else
          (Variables|Default|SetplayerLoc _returnvalue)
          (CallFunction|StartChasing))))
    (:NewEnumerator2
      (CallFunction|StopMovement))
    (:NewEnumerator3
      (CallFunction|TriggerLoseScreen))))

(fn ConstructionScript)
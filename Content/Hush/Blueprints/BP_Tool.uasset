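; BP_Tool is a wrench pickup that the player collects on interaction, but only while the character's NeedsTool flag is set.
; A construction-sized sphere shows a UI circle and prompt while the player overlaps without the tool, and hides them on exit.
; Pickup sets HasTool on the cached player, hides the wrench mesh and prints an electric box hint.
; ResetMesh makes the wrench visible again without clearing player flags.
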(event OnComponentBeginOverlap(Sphere)
  (params (OverlappedComponent :type Primitive%20Component%20Object%20Reference) (OtherActor :type Actor%20Object%20Reference) (OtherComp :type Primitive%20Component%20Object%20Reference) (OtherBodyIndex :type Integer) (bFromSweep :type Boolean) (SweepResult :type Hit%20Result%20Structure%20%28by%20ref%29))
  (bind _playerref (Variables|Default|GetPlayerRef))
  (if (and (== OtherActor _playerref) (not (Variables|/Game/ThirdPerson/Blueprints/BP_ThirdPersonCharacter.BP_ThirdPersonCharacter_C|GetbHasTool _playerref)))
    (CallFunction|ShowUI)))

(event OnComponentEndOverlap(Sphere)
  (params (OverlappedComponent :type Primitive%20Component%20Object%20Reference) (OtherActor :type Actor%20Object%20Reference) (OtherComp :type Primitive%20Component%20Object%20Reference) (OtherBodyIndex :type Integer))
  (if (== (Variables|Default|GetPlayerRef) OtherActor)
    (CallFunction|HideUI)))

(event Custom|ShowUI
  (Rendering|SetVisibility (Variables|Default|GetUICircle) true false)
  (Default|DisplayPrompt (Variables|Default|GetPlayerRef) "NewEnumerator0"))

(event Custom|HideUI
  (Rendering|SetVisibility (Variables|Default|GetUICircle) false false)
  (Default|HidePrompt (Variables|Default|GetPlayerRef) "NewEnumerator0"))

(event Custom|ResetMesh
  (Rendering|SetVisibility (Variables|Default|GetSM_Wrench) true false))

(event EventBeginPlay
  (bind _asbp_third_person_character (Utilities|Casting|CastToBP_ThirdPersonCharacter (Game|GetPlayerCharacter 0)))
  (Variables|Default|SetPlayerRef _asbp_third_person_character))

(event EventInteract
  (if (Variables|/Game/ThirdPerson/Blueprints/BP_ThirdPersonCharacter.BP_ThirdPersonCharacter_C|GetbNeedsTool (Variables|Default|GetPlayerRef))
    (Variables|/Game/ThirdPerson/Blueprints/BP_ThirdPersonCharacter.BP_ThirdPersonCharacter_C|SetbHasTool (Variables|Default|GetPlayerRef) true)
    (Rendering|SetVisibility (Variables|Default|GetSM_Wrench) false false)
    (CallFunction|HideUI)
    (Development|PrintString "Should find electric box")
    (else
      (Development|PrintString "Don't need this right now"))))

(fn ConstructionScript
  (Components|Sphere|SetSphereRadius (Variables|Default|GetSphere) (Variables|Public|GetIn%20Sphere%20Radius) true))
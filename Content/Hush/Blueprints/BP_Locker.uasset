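; Interactable hiding locker that moves the player in and out through scripted camera and door sequences.
; A trigger box toggles the UI circle and prompt, and Interact starts entry.
; Chained timelines lerp the player's FollowCamera between cached exterior, interior and original transforms, swinging the door 90 degrees between moves.
; The character's enter and leave sequences are called, and a separate LeaveLocker event reverses the trip without the exterior stop.
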(event OnComponentBeginOverlap(Box)
  (params (OverlappedComponent :type Primitive%20Component%20Object%20Reference) (OtherActor :type Actor%20Object%20Reference) (OtherComp :type Primitive%20Component%20Object%20Reference) (OtherBodyIndex :type Integer) (bFromSweep :type Boolean) (SweepResult :type Hit%20Result%20Structure%20%28by%20ref%29))
  (if (== OtherActor (Game|GetPlayerCharacter 0))
    (CallFunction|ShowUI)))

(event OnComponentEndOverlap(Box)
  (params (OverlappedComponent :type Primitive%20Component%20Object%20Reference) (OtherActor :type Actor%20Object%20Reference) (OtherComp :type Primitive%20Component%20Object%20Reference) (OtherBodyIndex :type Integer))
  (if (== (Game|GetPlayerCharacter 0) OtherActor)
    (CallFunction|HideUI)))

(event Custom|EnterLocker
  (bind _playercharacterref (Variables|Default|GetPlayerCharacterRef))
  (bind _exteriorcamtransform (Variables|Default|GetExteriorCamTransform))
  (bind _exteriorcamtransform_2 (Variables|Default|GetExteriorCamTransform))
  (bind _interiorcamtransform (Variables|Default|GetInteriorCamTransform))
  (bind _lockerdoorrot (Variables|Default|GetLockerDoorRot))
  (bind _lockerdoorrot_2 (Variables|Default|GetLockerDoorRot))
  (bind (_x _y) (Math|Vector|BreakVector (.location _exteriorcamtransform)))
  (bind (_roll _pitch _yaw) (Math|Rotator|BreakRotator _lockerdoorrot))
  (bind (_roll_2 _pitch_2 _yaw_2) (Math|Rotator|BreakRotator _lockerdoorrot_2))
  (bind _followcamera (Variables|/Game/ThirdPerson/Blueprints/BP_ThirdPersonCharacter.BP_ThirdPersonCharacter_C|GetFollowCamera _playercharacterref))
  (CallFunction|HideUI)
  (Variables|Default|SetMainCamTransform (Transformation|GetWorldTransform _followcamera))
  (Variables|Default|SetMainCamHeight (.z (Transformation|GetWorldLocation _followcamera)))
  (Variables|Default|SetbIsInsideLocker%20 true)
  (Default|EnterLockerSequence (Variables|Default|GetPlayerCharacterRef) self)
  (bind _alpha (Timeline|MoveToExtCam PlayFromStart)
    (:Update
      (Transformation|SetWorldLocationAndRotation (Variables|/Game/ThirdPerson/Blueprints/BP_ThirdPersonCharacter.BP_ThirdPersonCharacter_C|GetFollowCamera (Variables|Default|GetPlayerCharacterRef)) (Math|Vector|Lerp(Vector) (.location (Variables|Default|GetMainCamTransform)) (Math|Vector|MakeVector _x _y (Variables|Default|GetMainCamHeight)) _alpha) (Math|Rotator|Lerp(Rotator) (.rotation (Variables|Default|GetMainCamTransform)) (.rotation _exteriorcamtransform) _alpha true) false false))
    (:Finished
      (bind _alpha_2 (Timeline|OpenLockerDoor PlayFromStart)
        (:Update
          (Transformation|SetWorldRotation (Variables|Default|GetSM_LockerDoor1) (Math|Rotator|Lerp(Rotator) (Variables|Default|GetLockerDoorRot) (Math|Rotator|MakeRotator _roll _pitch (- _yaw 9e+01)) _alpha_2) false false))
        (:Finished
          (bind _alpha_3 (Timeline|ExtToIntCam PlayFromStart)
            (:Update
              (Transformation|SetWorldLocationAndRotation (Variables|/Game/ThirdPerson/Blueprints/BP_ThirdPersonCharacter.BP_ThirdPersonCharacter_C|GetFollowCamera (Variables|Default|GetPlayerCharacterRef)) (Math|Vector|Lerp(Vector) (.location _exteriorcamtransform_2) (.location _interiorcamtransform) _alpha_3) (Math|Rotator|Lerp(Rotator) (.rotation _exteriorcamtransform_2) (.rotation _interiorcamtransform) _alpha_3 true) false false))
            (:Finished
              (bind _alpha_4 (Timeline|CloseLockerDoor PlayFromStart)
                (:Update
                  (Transformation|SetWorldRotation (Variables|Default|GetSM_LockerDoor1) (Math|Rotator|Lerp(Rotator) (Math|Rotator|MakeRotator _roll_2 _pitch_2 (- _yaw_2 9e+01)) (Variables|Default|GetLockerDoorRot) _alpha_4) false false)
                  (Utilities|FlowControl|Delay 0.5)
                  (Default|DisplayPrompt (Variables|Default|GetPlayerCharacterRef) "NewEnumerator2"))))))))))

(event Custom|LeaveLocker
  (bind _lockerdoorrot (Variables|Default|GetLockerDoorRot))
  (bind _lockerdoorrot_2 (Variables|Default|GetLockerDoorRot))
  (bind _interiorcamtransform (Variables|Default|GetInteriorCamTransform))
  (bind _maincamtransform (Variables|Default|GetMainCamTransform))
  (bind (_roll _pitch _yaw) (Math|Rotator|BreakRotator _lockerdoorrot))
  (bind (_roll_2 _pitch_2 _yaw_2) (Math|Rotator|BreakRotator _lockerdoorrot_2))
  (bind (_location _rotation) (Math|Transform|BreakTransform _interiorcamtransform))
  (bind (_location_2 _rotation_2) (Math|Transform|BreakTransform _maincamtransform))
  (Default|HidePrompt (Variables|Default|GetPlayerCharacterRef) "NewEnumerator2")
  (Variables|Default|SetbIsInsideLocker%20 false)
  (bind _alpha (Timeline|OpenLockerDoorLeave PlayFromStart)
    (:Update
      (Transformation|SetWorldRotation (Variables|Default|GetSM_LockerDoor1) (Math|Rotator|Lerp(Rotator) (Variables|Default|GetLockerDoorRot) (Math|Rotator|MakeRotator _roll _pitch (- _yaw 9e+01)) _alpha) false false))
    (:Finished
      (bind _alpha_2 (Timeline|InttoNormCam PlayFromStart)
        (:Update
          (Transformation|SetWorldLocationAndRotation (Variables|/Game/ThirdPerson/Blueprints/BP_ThirdPersonCharacter.BP_ThirdPersonCharacter_C|GetFollowCamera (Variables|Default|GetPlayerCharacterRef)) (Math|Vector|Lerp(Vector) _location _location_2 _alpha_2) (Math|Rotator|Lerp(Rotator) _rotation _rotation_2 _alpha_2 true) false false))
        (:Finished
          (bind _alpha_3 (Timeline|CloseLockerDoorLeave PlayFromStart)
            (:Update
              (Transformation|SetWorldRotation (Variables|Default|GetSM_LockerDoor1) (Math|Rotator|Lerp(Rotator) (Math|Rotator|MakeRotator _roll_2 _pitch_2 (- _yaw_2 9e+01)) (Variables|Default|GetLockerDoorRot) _alpha_3) false false))
            (:Finished
              (Default|LeaveLockerSequence (Variables|Default|GetPlayerCharacterRef))
              (CallFunction|ShowUI))))))))

(event Custom|HideUI
  (Rendering|SetVisibility (Variables|Default|GetUICircle) false false)
  (Default|HidePrompt (Variables|Default|GetPlayerCharacterRef) "NewEnumerator1"))

(event Custom|ShowUI
  (Rendering|SetVisibility (Variables|Default|GetUICircle) true false)
  (Default|DisplayPrompt (Variables|Default|GetPlayerCharacterRef) "NewEnumerator1"))

(event EventBeginPlay
  (bind _asbp_third_person_character (Utilities|Casting|CastToBP_ThirdPersonCharacter (Game|GetPlayerCharacter 0)))
  (Variables|Default|SetPlayerCharacterRef _asbp_third_person_character)
  (Variables|Default|SetInteriorCamTransform (Transformation|GetWorldTransform (Variables|Default|GetInteriorCamera)))
  (Variables|Default|SetExteriorCamTransform (Transformation|GetWorldTransform (Variables|Default|GetExteriorCamera)))
  (Variables|Default|SetLockerDoorRot (Transformation|GetWorldRotation (Variables|Default|GetSM_LockerDoor1)))
  (Variables|Default|SetExteriorLeaveCamTransform (Transformation|GetWorldTransform (Variables|Default|GetExteriorCameraLeave))))

(event EventInteract
  (if (not (Variables|Default|GetbIsInsideLocker%20))
    (CallFunction|EnterLocker)))

(fn ConstructionScript)
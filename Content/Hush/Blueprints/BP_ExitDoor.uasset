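; BP_ExitDoor is the level exit door, gated by the player character's CanLeaveDoor flag.
; BeginPlay caches the third-person character, and the Box overlap toggles the UICircle marker for that player, plus an interaction prompt when leaving is allowed.
; Interact checks the same flag but only prints placeholder strings for either ending the game or needing a keypad.
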(event OnComponentBeginOverlap(Box)
  (params (OverlappedComponent :type Primitive%20Component%20Object%20Reference) (OtherActor :type Actor%20Object%20Reference) (OtherComp :type Primitive%20Component%20Object%20Reference) (OtherBodyIndex :type Integer) (bFromSweep :type Boolean) (SweepResult :type Hit%20Result%20Structure%20%28by%20ref%29))
  (if (== OtherActor (Variables|Default|GetPlayerRef))
    (CallFunction|ShowUI)))

(event OnComponentEndOverlap(Box)
  (params (OverlappedComponent :type Primitive%20Component%20Object%20Reference) (OtherActor :type Actor%20Object%20Reference) (OtherComp :type Primitive%20Component%20Object%20Reference) (OtherBodyIndex :type Integer))
  (if (== (Variables|Default|GetPlayerRef) OtherActor)
    (CallFunction|HideUI)))

(event Custom|ShowUI
  (bind _playerref (Variables|Default|GetPlayerRef))
  (Rendering|SetVisibility (Variables|Default|GetUICircle) true false)
  (if (Variables|/Game/ThirdPerson/Blueprints/BP_ThirdPersonCharacter.BP_ThirdPersonCharacter_C|GetbCanLeaveDoor _playerref)
    (Default|DisplayPrompt _playerref "NewEnumerator0")))

(event Custom|HideUI
  (bind _playerref (Variables|Default|GetPlayerRef))
  (Rendering|SetVisibility (Variables|Default|GetUICircle) false false)
  (if (Variables|/Game/ThirdPerson/Blueprints/BP_ThirdPersonCharacter.BP_ThirdPersonCharacter_C|GetbCanLeaveDoor _playerref)
    (Default|HidePrompt _playerref "NewEnumerator0")))

(event EventBeginPlay
  (bind _asbp_third_person_character (Utilities|Casting|CastToBP_ThirdPersonCharacter (Game|GetPlayerCharacter 0)))
  (Variables|Default|SetPlayerRef _asbp_third_person_character))

(event EventInteract
  (if (Variables|/Game/ThirdPerson/Blueprints/BP_ThirdPersonCharacter.BP_ThirdPersonCharacter_C|GetbCanLeaveDoor (Variables|Default|GetPlayerRef))
    (Development|PrintString "Leave game, reset and display enging screen")
    (else
      (Development|PrintString "needkeypad"))))

(fn ConstructionScript)
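; BP_Note is an interactable readable note that shows its text in a WB_Note widget.
; BeginPlay caches the third-person player and creates the widget from the note's text.
; Interact toggles reading, adding or removing the widget and calling the player's pick-up or put-down note sequence.
; A sphere trigger, sized in the construction script, shows or hides a billboard and player prompt, which are also hidden while reading.
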(event OnComponentBeginOverlap(Sphere)
  (params (OverlappedComponent :type Primitive%20Component%20Object%20Reference) (OtherActor :type Actor%20Object%20Reference) (OtherComp :type Primitive%20Component%20Object%20Reference) (OtherBodyIndex :type Integer) (bFromSweep :type Boolean) (SweepResult :type Hit%20Result%20Structure%20%28by%20ref%29))
  (if (== OtherActor (Variables|Default|GetPlayerRef))
    (CallFunction|ShowUI)))

(event OnComponentEndOverlap(Sphere)
  (params (OverlappedComponent :type Primitive%20Component%20Object%20Reference) (OtherActor :type Actor%20Object%20Reference) (OtherComp :type Primitive%20Component%20Object%20Reference) (OtherBodyIndex :type Integer))
  (if (== (Variables|Default|GetPlayerRef) OtherActor)
    (CallFunction|HideUI)))

(event Custom|ShowUI
  (Rendering|SetVisibility (Variables|Default|GetBillboard) true false)
  (Default|DisplayPrompt (Variables|Default|GetPlayerRef) "NewEnumerator0"))

(event Custom|HideUI
  (Rendering|SetVisibility (Variables|Default|GetBillboard) false false)
  (Default|HidePrompt (Variables|Default|GetPlayerRef) "NewEnumerator0"))

(event EventBeginPlay
  (bind _asbp_third_person_character (Utilities|Casting|CastToBP_ThirdPersonCharacter (Game|GetPlayerCharacter 0)))
  (Variables|Default|SetPlayerRef _asbp_third_person_character)
  (bind _returnvalue (UserInterface|CreateWidget "/Game/Hush/UI/WB_Note.WB_Note_C" 0 (Variables|Default|GetNoteText)))
  (Variables|Default|SetWBNote _returnvalue))

(event EventInteract
  (bind _playerref (Variables|Default|GetPlayerRef))
  (if (Variables|Default|GetbIsReadingNote)
    (Default|PutDownNoteSequence _playerref)
    (Variables|Default|SetbIsReadingNote (not (Variables|Default|GetbIsReadingNote)))
    (Widget|RemovefromParent (Variables|Default|GetWBNote))
    (CallFunction|ShowUI)
    (else
      (Default|PickUpNoteSequence _playerref)
      (Variables|Default|SetbIsReadingNote (not (Variables|Default|GetbIsReadingNote)))
      (UserInterface|Viewport|AddtoViewport (Variables|Default|GetWBNote) 0)
      (CallFunction|HideUI))))

(fn ConstructionScript
  (Components|Sphere|SetSphereRadius (Variables|Default|GetSphere) (Variables|Public|GetIn%20Sphere%20Radius) true))
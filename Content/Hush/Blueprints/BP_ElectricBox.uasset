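; BP_ElectricBox is an electric box the player repairs, provided they have the tool.
; A sphere, sized in the Construction Script, shows a circle indicator and player prompt on overlap while repair is pending, hiding both when the player leaves.
; The Repair event checks the cached player's HasTool flag, then sets HasRepaired on the player rather than the box and hides the UI, or prints a reminder to get the tool.
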(event OnComponentBeginOverlap(Sphere)
  (params (OverlappedComponent :type Primitive%20Component%20Object%20Reference) (OtherActor :type Actor%20Object%20Reference) (OtherComp :type Primitive%20Component%20Object%20Reference) (OtherBodyIndex :type Integer) (bFromSweep :type Boolean) (SweepResult :type Hit%20Result%20Structure%20%28by%20ref%29))
  (bind _playerref (Variables|Default|GetPlayerRef))
  (if (and (== OtherActor _playerref) (not (Variables|/Game/ThirdPerson/Blueprints/BP_ThirdPersonCharacter.BP_ThirdPersonCharacter_C|GetbHasRepaired _playerref)))
    (CallFunction|ShowUI)))

(event OnComponentEndOverlap(Sphere)
  (params (OverlappedComponent :type Primitive%20Component%20Object%20Reference) (OtherActor :type Actor%20Object%20Reference) (OtherComp :type Primitive%20Component%20Object%20Reference) (OtherBodyIndex :type Integer))
  (if (== (Variables|Default|GetPlayerRef) OtherActor)
    (CallFunction|HideUI)))

(event Custom|ShowUI
  (Rendering|SetVisibility (Variables|Default|GetUICircle) true false)
  (Default|DisplayPrompt (Variables|Default|GetPlayerRef) "NewEnumerator4"))

(event Custom|HideUI
  (Rendering|SetVisibility (Variables|Default|GetUICircle) false false)
  (Default|HidePrompt (Variables|Default|GetPlayerRef) "NewEnumerator4"))

(event EventBeginPlay
  (bind _asbp_third_person_character (Utilities|Casting|CastToBP_ThirdPersonCharacter (Game|GetPlayerCharacter 0)))
  (Variables|Default|SetPlayerRef _asbp_third_person_character))

(event EventRepair
  (if (Variables|/Game/ThirdPerson/Blueprints/BP_ThirdPersonCharacter.BP_ThirdPersonCharacter_C|GetbHasTool (Variables|Default|GetPlayerRef))
    (Development|PrintString "Repaired")
    (Variables|/Game/ThirdPerson/Blueprints/BP_ThirdPersonCharacter.BP_ThirdPersonCharacter_C|SetbHasRepaired (Variables|Default|GetPlayerRef) true)
    (CallFunction|HideUI)
    (else
      (Development|PrintString "Get TOOL"))))

(fn ConstructionScript
  (Components|Sphere|SetSphereRadius (Variables|Default|GetSphere) (Variables|Public|GetIn%20Sphere%20Radius) true))
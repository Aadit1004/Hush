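; BP_CeilingLight is a ceiling light actor whose spot light can be faded on and off.
; BeginPlay caches the SpotLight's intensity as the default level.
; TurnOnLight and TurnOffLight each play a timeline from the start, lerping the intensity between zero and that cached default.
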(event Custom|TurnOnLight
  (bind _alpha (Timeline|FadeOnLight PlayFromStart)
    (:Update
      (Rendering|Components|Light|SetIntensity (Variables|Default|GetSpotLight) (Math|Float|Lerp 0.0 (Variables|Default|GetDefaultLightIntensity) _alpha)))))

(event Custom|TurnOffLight
  (bind _alpha (Timeline|FadeOffLight PlayFromStart)
    (:Update
      (Rendering|Components|Light|SetIntensity (Variables|Default|GetSpotLight) (Math|Float|Lerp (Variables|Default|GetDefaultLightIntensity) 0.0 _alpha)))))

(event EventBeginPlay
  (Variables|Default|SetDefaultLightIntensity (Variables|/Script/Engine.LightComponentBase|GetIntensity (Variables|Default|GetSpotLight))))

(event Collision|EventActorBeginOverlap
  (params (OtherActor :type Actor%20Object%20Reference)))

(event EventTick
  (params (DeltaSeconds :type Float%20%28single-precision%29)))

(fn ConstructionScript)